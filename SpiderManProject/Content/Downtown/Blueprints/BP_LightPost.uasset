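; BP_LightPost is a configurable street light post prop for the Downtown environment, built entirely in its construction script with no runtime logic.
; Toggles remove the street lamps, street signs, electrical box and traffic light support beam, while selectors set sign mesh, sign yaw and beam mesh.
; One intensity value and an on/off switch drive both spotlights and the lamps' emissive dynamic materials, keeping glow and light in sync.
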(event EventBeginPlay)

(event Collision|EventActorBeginOverlap
  (params (OtherActor :type Actor%20Object%20Reference)))

(event EventTick
  (params (DeltaSeconds :type Float%20%28single-precision%29)))

(fn ConstructionScript
  (bind _signs (Variables|Default|GetSIgns))
  (bind _light_intensity (Variables|Default|GetLight%20Intensity))
  (bind _spotlight2 (Variables|Default|GetSpotLight2))
  ;[1 1 1] Setting up emissive material
  (bind _returnvalue (Rendering|Material|CreateDynamicMaterialInstance (Variables|Default|GetLightPostLamp1) 1 "/Game/Downtown/Materials/TrafficeLight_Emissive.TrafficeLight_Emissive" :!class /Script/Engine.PrimitiveComponent))
  (Variables|Default|SetLights1_DMI _returnvalue)
  (bind _returnvalue_2 (Rendering|Material|CreateDynamicMaterialInstance (Variables|Default|GetLightPostLamp2) 1 "/Game/Downtown/Materials/TrafficeLight_Emissive.TrafficeLight_Emissive" :!class /Script/Engine.PrimitiveComponent))
  (Variables|Default|SetLights2_DMI _returnvalue_2)
  ;[1 1 1] Street Signs Set up
  (Components|StaticMesh|SetStaticMesh _signs (Utilities|Array|Get(acopy) (LocalVariables|GetStreetSigns) (Math|Conversions|ToInteger(Byte) (Variables|Default|GetSigns_Mesh))))
  (if (Variables|Default|GetSign%20Toggle)
    _
    (else
      (Components|DestroyComponent _signs)))
  (Transformation|SetRelativeRotation _signs (Math|Rotator|MakeRotator 0.0 0.0 (Variables|Default|GetSign%20Rotation)) false false)
  ;[1 1 1] SupportBeam Length Selection
  (Components|StaticMesh|SetStaticMesh (Variables|Default|GetSupportBeam) (Utilities|Array|Get(acopy) (LocalVariables|GetSupportBeams) (Math|Conversions|ToInteger(Byte) (Variables|Default|GetSupportBeam_Mesh))))
  ;[1 1 1] Electrical Box Toggle
  (if (Variables|Default|GetElectricalBox_Toggle)
    _
    (else
      (Components|DestroyComponent (Variables|Default|GetElectricalBox))))
  ;[1 1 1] Support Beam Toggle
  (if (Variables|Default|GetTrafficLight%20SupportBeam)
    _
    (else
      (Components|DestroyComponent (Variables|Default|GetSupportBeam))))
  ;[1 1 1] Lights Toggle
  (if (Variables|Default|GetStreetLight%20Toggle)
    _
    (else
      (Components|DestroyComponent (Variables|Default|GetSpotLight1))))
  ;[1 1 1] Street Lights Values
  (if (Variables|Default|GetLight%20On/Off%20Toggle)
    (Rendering|Components|Light|SetIntensity _spotlight2 (* _light_intensity 1e+04))
    (Rendering|Material|SetScalarParameterValue (Variables|Default|GetLights1_DMI) "EmissiveStrength" _light_intensity :!class /Script/Engine.MaterialInstanceDynamic)
    (else
      (Rendering|Components|Light|SetIntensity _spotlight2 0.0)
      (Rendering|Material|SetScalarParameterValue (Variables|Default|GetLights1_DMI) "EmissiveStrength" 0.0 :!class /Script/Engine.MaterialInstanceDynamic))))