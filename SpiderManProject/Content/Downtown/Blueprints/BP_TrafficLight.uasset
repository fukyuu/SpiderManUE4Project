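; Placeable traffic light that cycles endlessly through red, green and yellow from BeginPlay.
; The construction script creates a dynamic material instance on the static mesh, and the event graph lights each lamp through its scalar parameters.
; Looping Delay chains time the phases from TrafficLightLength, carving the Yellow duration out of green.
; The Offset flag starts the cycle on red instead of green, so lights can alternate with traffic flow.
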(event EventBeginPlay
  (bind _traffic_light_length (Variables|Default|GetTraffic%20Light%20Length))
  (bind _lights (Variables|Default|GetLIghts))
  (bind _yellow (Variables|Default|GetYellow))
  (bind _lights_2 (Variables|Default|GetLIghts))
  (bind _lights_3 (Variables|Default|GetLIghts))
  (bind _returnvalue (* _traffic_light_length 5.0))
  (bind _returnvalue_2 (- _returnvalue _yellow))
  ;[1 1 1] Place in level, and turn it on/off depending on traffic flow.
  (if (Variables|Default|GetOffset)
    ;[1 1 1] Red
    (Rendering|Material|SetScalarParameterValue _lights "Red" 25.0 :!class /Script/Engine.MaterialInstanceDynamic :!label _label)
    (Rendering|Material|SetScalarParameterValue _lights "Green" 0.0 :!class /Script/Engine.MaterialInstanceDynamic)
    (Rendering|Material|SetScalarParameterValue _lights "Yellow" 0.0 :!class /Script/Engine.MaterialInstanceDynamic)
    (Utilities|FlowControl|Delay _returnvalue)
    ;[1 1 1] Green
    (Rendering|Material|SetScalarParameterValue _lights_2 "Red" 0.0 :!class /Script/Engine.MaterialInstanceDynamic)
    (Rendering|Material|SetScalarParameterValue _lights_2 "Green" 25.0 :!class /Script/Engine.MaterialInstanceDynamic)
    (Rendering|Material|SetScalarParameterValue _lights_2 "Yellow" 0.0 :!class /Script/Engine.MaterialInstanceDynamic)
    (Utilities|FlowControl|Delay _returnvalue_2)
    ;[1 1 1] Yellow
    (Rendering|Material|SetScalarParameterValue _lights_3 "Red" 0.0 :!class /Script/Engine.MaterialInstanceDynamic)
    (Rendering|Material|SetScalarParameterValue _lights_3 "Green" 0.0 :!class /Script/Engine.MaterialInstanceDynamic)
    (Rendering|Material|SetScalarParameterValue _lights_3 "Yellow" 25.0 :!class /Script/Engine.MaterialInstanceDynamic)
    (Utilities|FlowControl|Delay _yellow)
    (goto _label)
    (else
      ;[1 1 1] Green
      (Rendering|Material|SetScalarParameterValue _lights "Red" 0.0 :!class /Script/Engine.MaterialInstanceDynamic :!label _label_2)
      (Rendering|Material|SetScalarParameterValue _lights "Green" 25.0 :!class /Script/Engine.MaterialInstanceDynamic)
      (Rendering|Material|SetScalarParameterValue _lights "Yellow" 0.0 :!class /Script/Engine.MaterialInstanceDynamic)
      (Utilities|FlowControl|Delay _returnvalue_2)
      ;[1 1 1] Yellow
      (Rendering|Material|SetScalarParameterValue _lights_2 "Red" 0.0 :!class /Script/Engine.MaterialInstanceDynamic)
      (Rendering|Material|SetScalarParameterValue _lights_2 "Green" 0.0 :!class /Script/Engine.MaterialInstanceDynamic)
      (Rendering|Material|SetScalarParameterValue _lights_2 "Yellow" 25.0 :!class /Script/Engine.MaterialInstanceDynamic)
      (Utilities|FlowControl|Delay _yellow)
      ;[1 1 1] Red
      (Rendering|Material|SetScalarParameterValue _lights_3 "Red" 25.0 :!class /Script/Engine.MaterialInstanceDynamic)
      (Rendering|Material|SetScalarParameterValue _lights_3 "Green" 0.0 :!class /Script/Engine.MaterialInstanceDynamic)
      (Rendering|Material|SetScalarParameterValue _lights_3 "Yellow" 0.0 :!class /Script/Engine.MaterialInstanceDynamic)
      (Utilities|FlowControl|Delay _returnvalue)
      (goto _label_2))))

(fn ConstructionScript
  (bind _returnvalue (Rendering|Material|CreateDynamicMaterialInstance (Variables|Default|GetStaticMesh) 0 "/Game/Downtown/Materials/TrafficLight.TrafficLight" :!class /Script/Engine.PrimitiveComponent))
  (Variables|Default|SetLIghts _returnvalue))